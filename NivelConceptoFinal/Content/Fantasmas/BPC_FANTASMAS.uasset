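; Ghost enemy pawn for a Pac-Man-style game that roams, chases the player and takes lives.
; After a start delay it loops AI moves to random reachable points, repeating on success or failure.
; Tick and pawn sensing share a chase branch gated by PersecucionJugador, which this graph never sets; failed chases resume roaming after a retriggerable delay.
; Overlapping its hit collision decrements the player's Vidas and calls PacManDeath.
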(event OnSeePawn(PawnSensing)
  (params (Pawn :type Pawn%20Object%20Reference))
  (if (Variables|Default|GetPersecucionJugador)
    (bind _asbp_third_person_character (Utilities|Casting|CastToBP_ThirdPersonCharacter (Game|GetPlayerCharacter 0)))
    (AI|AIMoveTo self "0, 0, 0" _asbp_third_person_character 5.0 false
      (:OnFail
        (Utilities|FlowControl|RetriggerableDelay 3.0)
        (CallFunction|Randomroam)))))

(event OnComponentBeginOverlap(Golpecollision)
  (params (OverlappedComponent :type Primitive%20Component%20Object%20Reference) (OtherActor :type Actor%20Object%20Reference) (OtherComp :type Primitive%20Component%20Object%20Reference) (OtherBodyIndex :type Integer) (bFromSweep :type Boolean) (SweepResult :type Hit%20Result%20Structure%20%28by%20ref%29))
  (bind _asbp_third_person_character (Utilities|Casting|CastToBP_ThirdPersonCharacter OtherActor))
  (bind _output_get (Variables|Default|SetThird%20Person%20Character _asbp_third_person_character))
  (Variables|/Game/ThirdPerson/Blueprints/BP_ThirdPersonCharacter.BP_ThirdPersonCharacter_C|SetVidas _output_get (- (Variables|/Game/ThirdPerson/Blueprints/BP_ThirdPersonCharacter.BP_ThirdPersonCharacter_C|GetVidas _output_get) 1))
  (Default|PacManDeath (Variables|Default|GetThird%20Person%20Character)))

(event Custom|Randomroam
  (AI|AIMoveTo self (.RandomLocation (AI|Navigation|GetRandomReachablePointinRadius (Transformation|GetActorLocation) 3e+03 0 0)) 0 5.0 false
    (:OnSuccess
      _)
    (:OnFail
      _))
  (CallFunction|Randomroam))

(event EventBeginPlay
  (Utilities|FlowControl|Delay 5.0)
  (CallFunction|Randomroam))

(event Collision|EventActorBeginOverlap
  (params (OtherActor :type Actor%20Object%20Reference)))

(event EventTick
  (params (DeltaSeconds :type Float%20%28single-precision%29))
  (if (Variables|Default|GetPersecucionJugador)
    (bind _asbp_third_person_character (Utilities|Casting|CastToBP_ThirdPersonCharacter (Game|GetPlayerCharacter 0)))
    (AI|AIMoveTo self "0, 0, 0" _asbp_third_person_character 5.0 false
      (:OnFail
        (Utilities|FlowControl|RetriggerableDelay 3.0)
        (CallFunction|Randomroam)))))

(fn ConstructionScript)