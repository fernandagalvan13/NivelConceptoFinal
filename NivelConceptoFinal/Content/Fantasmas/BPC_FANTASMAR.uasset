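; Ghost enemy in a Pac-Man style game that roams, chases or flees the player, and costs a life on contact.
; After a start delay it loops AIMoveTo to random reachable points.
; Tick and PawnSensing share one branch: PersecucionJugador selects pursuit, or flight at a set speed when IsScared, otherwise delayed roaming.
; Hit-collision overlap destroys a scared ghost, or triggers PacManDeath unless the shield is active; the coin reward is unconnected.
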(event OnSeePawn(PawnSensing)
  (params (Pawn :type Pawn%20Object%20Reference))
  (bind _returnvalue (Game|GetPlayerCharacter 0))
  (bind _self self)
  ;[0.15 0.15 0.15 0.5] Persecución
  (if (Variables|Default|GetPersecucionJugador)
    (bind _asbp_third_person_character (Utilities|Casting|CastToBP_ThirdPersonPacman _returnvalue))
    (if (Variables|Default|GetIsScared?)
      (Variables|/Script/Engine.CharacterMovementComponent|SetMaxWalkSpeed (Variables|Character|GetCharacterMovement) 4e+02)
      (AI|AIMoveTo _self (* (- (Transformation|GetActorLocation) (Transformation|GetActorLocation _returnvalue)) 1.0) 0 5.0 false)
      (else
        (AI|AIMoveTo _self "0, 0, 0" _asbp_third_person_character 5.0 false)))
    (else
      (Utilities|FlowControl|RetriggerableDelay 3.0)
      (CallFunction|Randomroam))))

(event OnComponentBeginOverlap(Golpecollision)
  (params (OverlappedComponent :type Primitive%20Component%20Object%20Reference) (OtherActor :type Actor%20Object%20Reference) (OtherComp :type Primitive%20Component%20Object%20Reference) (OtherBodyIndex :type Integer) (bFromSweep :type Boolean) (SweepResult :type Hit%20Result%20Structure%20%28by%20ref%29))
  ;[0.15 0.15 0.15 0.5] Golpe
  (bind _asbp_third_person_character (Utilities|Casting|CastToBP_ThirdPersonPacman OtherActor))
  (bind _output_get (Variables|Default|SetThird%20Person%20Character _asbp_third_person_character))
  (if (Variables|Default|GetIsScared?)
    (Actor|DestroyActor)
    (elif (not (Variables|/Game/ThirdPerson/Blueprints/BP_ThirdPersonPacman.BP_ThirdPersonPacman_C|GetEscudoActivo (Variables|Default|GetThird%20Person%20Character)))
      (Variables|/Game/ThirdPerson/Blueprints/BP_ThirdPersonPacman.BP_ThirdPersonPacman_C|SetVidas _output_get (- (Variables|/Game/ThirdPerson/Blueprints/BP_ThirdPersonPacman.BP_ThirdPersonPacman_C|GetVidas _output_get) 1))
      (Default|PacManDeath (Variables|Default|GetThird%20Person%20Character)))))

(event Custom|Randomroam
  ;[0.15 0.15 0.15 0.5] Vista
  (AI|AIMoveTo self (.RandomLocation (AI|Navigation|GetRandomReachablePointinRadius (Transformation|GetActorLocation) 3e+03 0 0)) 0 5.0 false
    (:OnSuccess
      _)
    (:OnFail
      _))
  (CallFunction|Randomroam))

(event EventBeginPlay
  ;[0.15 0.15 0.15 0.5] Activa
  (Utilities|FlowControl|Delay 1e+01)
  (CallFunction|Randomroam))

(event Collision|EventActorBeginOverlap
  (params (OtherActor :type Actor%20Object%20Reference)))

(event EventTick
  (params (DeltaSeconds :type Float%20%28single-precision%29))
  (bind _returnvalue (Game|GetPlayerCharacter 0))
  (bind _self self)
  ;[0.15 0.15 0.15 0.5] Persecución
  (if (Variables|Default|GetPersecucionJugador)
    (bind _asbp_third_person_character (Utilities|Casting|CastToBP_ThirdPersonPacman _returnvalue))
    (if (Variables|Default|GetIsScared?)
      (Variables|/Script/Engine.CharacterMovementComponent|SetMaxWalkSpeed (Variables|Character|GetCharacterMovement) 4e+02)
      (AI|AIMoveTo _self (* (- (Transformation|GetActorLocation) (Transformation|GetActorLocation _returnvalue)) 1.0) 0 5.0 false)
      (else
        (AI|AIMoveTo _self "0, 0, 0" _asbp_third_person_character 5.0 false)))
    (else
      (Utilities|FlowControl|RetriggerableDelay 3.0)
      (CallFunction|Randomroam))))

(fn ConstructionScript)